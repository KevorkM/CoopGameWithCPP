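; BP_OpenWithKey is a two-leaf door that opens when the F key is pressed near it; no key item is checked.
; Overlapping the collision as an SCharacter shows a text prompt and allows opening, and leaving reverses both.
; Two separate F handlers each play a timeline that sets one leaf's yaw.
; Opening sets a flag that keeps the prompt from reappearing, and nothing closes the doors.
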(event OnComponentBeginOverlap(Collision)
  (params (OverlappedComponent :type Primitive%20Component%20Object%20Reference) (OtherActor :type Actor%20Object%20Reference) (OtherComp :type Primitive%20Component%20Object%20Reference) (OtherBodyIndex :type Integer) (bFromSweep :type Boolean) (SweepResult :type Hit%20Result%20Structure%20%28by%20ref%29))
  ;[1 1 1] Show/Hide To open door
  (Utilities|Casting|CastToSCharacter OtherActor)
  (if (not (Variables|Default|GetHasDoorBeenOpened?))
    (Rendering|SetVisibility (Variables|Default|GetTextRender) true false)
    (Variables|Default|SetCanOpenDoor? true)))

(event OnComponentEndOverlap(Collision)
  (params (OverlappedComponent :type Primitive%20Component%20Object%20Reference) (OtherActor :type Actor%20Object%20Reference) (OtherComp :type Primitive%20Component%20Object%20Reference) (OtherBodyIndex :type Integer))
  ;[1 1 1] Show/Hide To open door
  (Utilities|Casting|CastToSCharacter OtherActor)
  (Rendering|SetVisibility (Variables|Default|GetTextRender) false false)
  (Variables|Default|SetCanOpenDoor? false))

(event Input|KeyboardEvents|F
  (params (Key :type Key%20Structure))
  (:Pressed
    (if (Variables|Default|GetCanOpenDoor?)
      (Variables|Default|SetHasDoorBeenOpened? true)
      (bind _doorrotation (Timeline|Timeline_0 Play)
        (:Update
          (Transformation|SetRelativeRotation (Variables|Default|GetDoor2) (Math|Rotator|MakeRotator 0.0 0.0 _doorrotation) false false))))))

(event Input|KeyboardEvents|F
  (params (Key :type Key%20Structure))
  ;[1 1 1] Opening Right door
  (:Pressed
    (if (Variables|Default|GetCanOpenDoor?)
      (Rendering|SetVisibility (Variables|Default|GetTextRender) false false)
      (Variables|Default|SetHasDoorBeenOpened? true)
      (bind _doorrotation (Timeline|Open%20Door Play)
        (:Update
          (Transformation|SetRelativeRotation (Variables|Default|GetDoor) (Math|Rotator|MakeRotator 0.0 0.0 _doorrotation) false false))))))

(fn ConstructionScript)