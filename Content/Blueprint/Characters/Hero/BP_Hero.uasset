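; BP_Hero is the hero character Blueprint, handling HUD setup, noise emission and debug feedback.
; On BeginPlay it clears the current weapon and adds a crosshair widget to the viewport.
; Every Tick it emits pawn noise with itself as noise maker.
; Debug hooks print the key count when 1 is pressed and draw each health delta at the actor's location.
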(event OnHealthChanged(Health1)
  (params (OwningHealthComp :type Health%20Component%20Object%20Reference) (Health :type Float%20%28single-precision%29) (HealthDelta :type Float%20%28single-precision%29) (DamageType :type Damage%20Type%20Object%20Reference) (InstigatedBy :type Controller%20Object%20Reference) (DamageCauser :type Actor%20Object%20Reference))
  (Rendering|Debug|DrawDebugString (Transformation|GetActorLocation) (Utilities|String|ToString(Float) HealthDelta) 0 "(R=1.000000,G=1.000000,B=1.000000,A=1.000000)" 1.0))

(event EventBeginPlay
  (Utilities|FlowControl|Sequence
    (:then_0
      (Variables|Default|SetCurrentWeapon_0 0)
      (bind _returnvalue (UserInterface|CreateWidget "/Game/Blueprint/Widgets/WBP_Crosshair.WBP_Crosshair_C"))
      (UserInterface|Viewport|AddtoViewport _returnvalue 0))))

(event EventTick
  (params (DeltaSeconds :type Float%20%28single-precision%29))
  (Class|Pawn|PawnMakeNoise 0.0 "0, 0, 0" true self))

(event Input|KeyboardEvents|1
  (params (Key :type Key%20Structure))
  (:Pressed
    (Development|PrintString (Utilities|String|ToString(Integer) (Variables|Default|GetNumberOfKey)))))

(fn ConstructionScript)