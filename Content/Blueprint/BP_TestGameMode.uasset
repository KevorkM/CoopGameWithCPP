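; Test game mode that spawns AI bots at locations chosen by an environment query.
; SpawnNewBot runs EQS_FindSpawnLocation in random-best-25% mode and binds to its completion event.
; Each returned location gets a debug sphere and a random choice of BP_AdvanceAI or BP_STrackerBot2, adjusted to avoid collisions or skipped.
; The query status check is disconnected, so results are used without checking success.
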(event Custom|OnQueryFinishedEvent_Event_0
  (params (QueryInstance :type Env%20Query%20Instance%20Blueprint%20Wrapper%20Object%20Reference) (QueryStatus :type EEnvQueryStatus%20Enum :default "Processing"))
  (bind _resultlocations (AI|EQS|GetQueryResultsasLocations QueryInstance))
  (for _array_element _resultlocations
    (Rendering|Debug|DrawDebugSphere _array_element 5e+01 12 "(R=1.000000,G=0.064122,B=0.326501,A=1.000000)" 2.0 2.0)
    (Game|SpawnActorfromClass (select (Math|Random|RandomBool) "/Game/Blueprint/BP_AdvanceAI.BP_AdvanceAI_C" "/Game/Blueprint/BP_STrackerBot2.BP_STrackerBot2_C") (Math|Transform|MakeTransform _array_element) "AdjustIfPossibleButDontSpawnIfColliding" 0 0)))

(event EventSpawnNewBot
  (bind _returnvalue (AI|EQS|RunEQSQuery "/Game/Blueprint/EQS_FindSpawnLocation.EQS_FindSpawnLocation" self "RandomBest25Pct"))
  (EventDispatchers|AssignOnQueryFinishedEvent _returnvalue (delegate Custom|OnQueryFinishedEvent_Event_0)))

(fn ConstructionScript)